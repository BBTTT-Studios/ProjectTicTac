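; BP_Marker is a grabbable VR whiteboard marker that paints on BP_Canvas actors.
; While held or always tracing, it line-traces from the tip each tick, passing hit UV, brush texture and size to the canvas's DrawBrush.
; Hitting a BP_PaintSelect adopts its texture and updates the dynamic-material preview.
; Pickup and Drop toggle physics, attachment and input; the right thumbstick's Y axis adjusts brush size and its text readout.
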(event EventBeginPlay
  ;[1 1 1] Setting BrushSize indicator and texture preview material
  (Rendering|Components|TextRender|SetText (Variables|Default|GetTextRender) (Utilities|Text|ToText(Float) (Variables|Default|GetBrushSize) "HalfToEven"))
  (bind _returnvalue (Rendering|Material|CreateDynamicMaterialInstance "/Game/Blueprints/Whiteboard2/M_Brush.M_Brush" "None" :!class /Script/Engine.KismetMaterialLibrary))
  (bind _output_get (Variables|Default|SetBrushPreview _returnvalue))
  (Rendering|Material|SetTextureParameterValue _output_get "BrushTexture" (Variables|Default|GetBrushTexture))
  (Rendering|Material|SetMaterial (Variables|Default|GetPlane) 0 (Variables|Default|GetBrushPreview)))

(event EventTick
  (params (DeltaSeconds :type Float%20%28single-precision%29))
  (bind _markertip (Variables|Default|GetMarkerTip))
  (bind _returnvalue (Transformation|GetWorldLocation _markertip))
  ;[1 1 1] Check each tick to see if the linetrace is hitting anything
  (if (Variables|Default|GetAlwaysTracing)
    (bind _outhit (Collision|LineTraceByChannel _returnvalue (+ _returnvalue (* (Math|Vector|GetUpVector _markertip) (Variables|Default|GetTraceDistance))) "TraceTypeQuery1" true 0 "ForOneFrame" :!label _label))
    ;[1 1 1] If trace hits an instance of BP_Canvas, call Draw function on it
    (bind _asbp_canvas (Utilities|Casting|CastToBP_Canvas (.HitActor (Collision|BreakHitResult _outhit)))
      (:then
        (Default|DrawBrush _asbp_canvas (Variables|Default|GetBrushTexture) (Variables|Default|GetBrushSize) (.UV (Class|GameplayStatics|FindCollisionUV _outhit))))
      (:CastFailed
        ;[1 1 1] If Linetrace hits an instance of BP_PaintSelect, get it's texture and apply to Marker
        (bind _asbp_paint_select (Utilities|Casting|CastToBP_PaintSelect (.HitActor (Collision|BreakHitResult _outhit))))
        (bind _output_get (Variables|Default|SetBrushTexture (Variables|/Game/Blueprints/Whiteboard2/BP_PaintSelect.BP_PaintSelect_C|GetTexture _asbp_paint_select)))
        (Rendering|Material|SetTextureParameterValue (Variables|Default|GetBrushPreview) "BrushTexture" _output_get)))
    (elif (Variables|Default|GetIsHeld)
      (goto _label))))

(event EventPickup
  (params (AttachTo :type Scene%20Component%20Object%20Reference))
  ;[1 1 1] Handle Pickup and Drop events
  (Variables|Default|SetIsHeld true)
  (Physics|SetSimulatePhysics (Variables|Default|GetMarker) false)
  (Transformation|AttachComponentToComponent (VehicleSound|GetRootComponent) AttachTo "None" "KeepWorld" "KeepWorld" "KeepWorld" false)
  (Input|EnableInput (Game|GetPlayerController 0)))

(event EventDrop
  ;[1 1 1] Handle Pickup and Drop events
  (Variables|Default|SetIsHeld false)
  (Physics|SetSimulatePhysics (Variables|Default|GetMarker) true)
  (Transformation|DetachFromActor "KeepWorld" "KeepWorld" "KeepWorld")
  (Input|DisableInput (Game|GetPlayerController 0)))

(event Input|AxisEvents|InputAxisMotionControllerThumbRight_Y
  (params (AxisValue :type Float%20%28single-precision%29))
  (bind _returnvalue (Input|AxisValues|GetMotionControllerThumbRight_X))
  ;[1 1 1] Adjust Brush Draw Size
  (if (and (and (< _returnvalue 0.25) (> _returnvalue -0.25)) (or (> AxisValue 0.25) (< AxisValue -0.25)))
    (bind _output_get (Variables|Default|SetBrushSize (Math|Conversions|ToFloat(Integer) (Math|Float|Round (Math|Float|Clamp(Float) (+ (* AxisValue 1.0) (Variables|Default|GetBrushSize)) 1.0 2e+02)))))
    ;;[1 1 1] Update brush size indicator text
    (Rendering|Components|TextRender|SetText (Variables|Default|GetTextRender) (Utilities|Text|ToText(Float) _output_get "HalfToEven"))))

(fn ConstructionScript)