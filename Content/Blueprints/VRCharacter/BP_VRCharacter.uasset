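; VR player character that combines roomscale headset tracking with left-thumbstick locomotion.
; Each tick shifts the PlayerCollision capsule by the headset's horizontal movement since the last update.
; It then repositions the actor from the capsule location minus the headset's horizontal offset, with a height adjustment from capsule half-height.
; Thumbstick axes offset the capsule along camera forward/right with Z zeroed, unswept and unscaled by delta time.
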(event Custom|UpdateRoomscalePosition
  (bind _deviceposition (Class|HeadMountedDisplayFunctionLibrary|GetOrientationandPosition))
  (bind (_x _y) (Math|Vector|BreakVector _deviceposition))
  (bind _returnvalue (Math|Vector|MakeVector _x _y 0.0))
  (Transformation|AddWorldOffset (Variables|Default|GetPlayerCollision) (- _returnvalue (Variables|Default|GetLastRoomScalePosition)) false false)
  (Variables|Default|SetLastRoomScalePosition _returnvalue))

(event Custom|UpdateActorLocation
  (bind _deviceposition (Class|HeadMountedDisplayFunctionLibrary|GetOrientationandPosition))
  (bind (_x _y) (Math|Vector|BreakVector _deviceposition))
  (Transformation|SetActorLocation (- (Transformation|GetWorldLocation (Variables|Default|GetPlayerCollision)) (Math|Vector|MakeVector _x _y (+ (* (Variables|/Script/Engine.CapsuleComponent|GetCapsuleHalfHeight (Variables|Default|GetPlayerCollision)) -1.0) 44.0))) false false))

(event EventBeginPlay)

(event Collision|EventActorBeginOverlap
  (params (OtherActor :type Actor%20Object%20Reference)))

(event EventTick
  (params (DeltaSeconds :type Float%20%28single-precision%29))
  (CallFunction|UpdateRoomscalePosition)
  (CallFunction|UpdateActorLocation))

(event Input|AxisEvents|InputAxisMotionControllerThumbLeft_Y
  (params (AxisValue :type Float%20%28single-precision%29))
  (bind _returnvalue (* AxisValue 4.0))
  (bind _camera (Variables|Default|GetCamera))
  (bind _returnvalue_2 (Math|Vector|GetForwardVector _camera))
  (bind _returnvalue_3 (* _returnvalue_2 _returnvalue))
  (Transformation|AddLocalOffset (Variables|Default|GetPlayerCollision) (Math|Vector|MakeVector (.x _returnvalue_3) (.y _returnvalue_3) 0.0) false false))

(event Input|AxisEvents|InputAxisMotionControllerThumbLeft_X
  (params (AxisValue :type Float%20%28single-precision%29))
  (bind _returnvalue (* AxisValue 4.0))
  (bind _camera (Variables|Default|GetCamera))
  (bind _returnvalue_2 (Math|Vector|GetRightVector _camera))
  (bind _returnvalue_3 (* _returnvalue_2 _returnvalue))
  (Transformation|AddLocalOffset (Variables|Default|GetPlayerCollision) (Math|Vector|MakeVector (.x _returnvalue_3) (.y _returnvalue_3) 0.0) false false))

(fn ConstructionScript)