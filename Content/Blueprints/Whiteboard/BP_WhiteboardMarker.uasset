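; BP_WhiteboardMarker is a holdable marker that draws on a BP_Whiteboard.
; Pickup disables physics on its cube and attaches it to the given component with a rotated grip, while Drop detaches it and restores physics.
; While held, Tick runs a short complex trace along the Sphere's up vector, shown with debug lines.
; On a whiteboard hit, it passes the collision UV to DrawOnWhiteboard.
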(event EventTick
  (params (DeltaSeconds :type Float%20%28single-precision%29))
  (bind _sphere (Variables|Default|GetSphere))
  (bind _returnvalue (Transformation|GetWorldLocation _sphere))
  (if (Variables|Default|GetIsHeld)
    (bind (_outhit _returnvalue_2) (Collision|LineTraceByChannel _returnvalue (+ _returnvalue (* (Math|Vector|GetUpVector _sphere) 13.0)) "TraceTypeQuery1" true 0 "ForOneFrame"))
    (if _returnvalue_2
      (bind _asbp_whiteboard (Utilities|Casting|CastToBP_Whiteboard (.HitActor (Collision|BreakHitResult _outhit))))
      (Default|DrawonWhiteboard _asbp_whiteboard (.UV (Class|GameplayStatics|FindCollisionUV _outhit))))))

(event Collision|EventActorBeginOverlap
  (params (OtherActor :type Actor%20Object%20Reference)))

(event EventBeginPlay)

(event EventPickup
  (params (AttachTo :type Scene%20Component%20Object%20Reference))
  (Variables|Default|SetIsHeld true)
  (Physics|SetSimulatePhysics (Variables|Default|GetCube) false)
  (Transformation|AttachComponentToComponent (VehicleSound|GetRootComponent) AttachTo "None" "SnapToTarget" "SnapToTarget" "KeepWorld" false)
  (Transformation|AddLocalRotation (Variables|Default|GetDefaultSceneRoot) "-110.000000, 0,-60.000000" false false))

(event EventDrop
  (Variables|Default|SetIsHeld false)
  (Physics|SetSimulatePhysics (Variables|Default|GetCube) true)
  (Transformation|DetachFromActor "KeepWorld" "KeepWorld" "KeepWorld"))

(fn ConstructionScript)