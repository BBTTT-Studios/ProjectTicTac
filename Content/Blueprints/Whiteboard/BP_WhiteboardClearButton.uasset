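; VR push button, named for clearing the whiteboard, that calls I_Use on its linked object when fully pressed.
; An overlapping motion controller starts tracking, and each tick projects its movement onto the button's up axis to set clamped depression.
; Full travel fires the action, raises material glow and plays a sound.
; The button then eases back with VInterpTo, as it does when contact ends, and resets glow at rest.
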(event OnComponentBeginOverlap(Button)
  (params (OverlappedComponent :type Primitive%20Component%20Object%20Reference) (OtherActor :type Actor%20Object%20Reference) (OtherComp :type Primitive%20Component%20Object%20Reference) (OtherBodyIndex :type Integer) (bFromSweep :type Boolean) (SweepResult :type Hit%20Result%20Structure%20%28by%20ref%29))
  (if (and (not (Variables|Default|GetbIsTracking)) (not (Variables|Default|GetbIsReturning)))
    (bind _asbp_motion_controller (Utilities|Casting|CastToBP_MotionController OtherActor))
    (Variables|Default|SetMotionControllerRef (Variables|/Game/VirtualRealityBP/Blueprints/BP_MotionController.BP_MotionController_C|GetMotionController _asbp_motion_controller))
    (Variables|Default|SetbIsTracking true)
    (Variables|Default|SetMCInitialLocation (Transformation|GetWorldLocation (Variables|Default|GetMotionControllerRef)))
    (Variables|Default|SetButtonInitialLocation (Transformation|GetWorldLocation (Variables|Default|GetButton)))))

(event OnComponentEndOverlap(Button)
  (params (OverlappedComponent :type Primitive%20Component%20Object%20Reference) (OtherActor :type Actor%20Object%20Reference) (OtherComp :type Primitive%20Component%20Object%20Reference) (OtherBodyIndex :type Integer))
  (bind _asbp_motion_controller (Utilities|Casting|CastToBP_MotionController OtherActor))
  (if (== (Variables|/Game/VirtualRealityBP/Blueprints/BP_MotionController.BP_MotionController_C|GetMotionController _asbp_motion_controller) (Variables|Default|GetMotionControllerRef))
    (Variables|Default|SetbIsTracking false)
    (Variables|Default|SetbIsReturning true)))

(event Custom|Fully%20Pressed
  (Rendering|Material|SetScalarParameterValue (Variables|Default|GetMaterialInstanceButton) "Glow" (Variables|Default|GetGlowIntensity) :!class /Script/Engine.MaterialInstanceDynamic)
  (Variables|Default|SetbIsTracking false)
  (Variables|Default|SetbIsReturning true)
  (CallFunction|ButtonAction)
  (Audio|PlaySoundatLocation "/Game/Blueprints/Button/Boop.Boop" (Transformation|GetWorldLocation (Variables|Default|GetDefaultSceneRoot)) "0, 0, 0" 1.0 1.0 0.0 0 0 0))

(event Custom|ButtonAction
  ;[0.09121 1 0] Button Action
  (bind _asi_use (Utilities|Casting|CastToI_Use (Variables|Default|GetLinkedObject)))
  (Default|Use _asi_use))

(event EventTick
  (params (DeltaSeconds :type Float%20%28single-precision%29))
  (if (Variables|Default|GetbIsTracking)
    (Variables|Default|SetCurrentButtonTravel (Math|Float|Clamp(Float) (Math|Float|Absolute(Float) (Math|Vector|VectorLength (Math|Vector|ProjectVectorontoVector (- (Transformation|GetWorldLocation (Variables|Default|GetMotionControllerRef)) (Variables|Default|GetMCInitialLocation)) (Math|Vector|GetUpVector (Variables|Default|GetButton))))) 0.0 (Variables|Default|GetMaximumButtonTravel)))
    (Transformation|SetWorldLocation (Variables|Default|GetButton) (- (Variables|Default|GetButtonInitialLocation) (* (Math|Vector|GetUpVector (Variables|Default|GetButton)) (Variables|Default|GetCurrentButtonTravel))) false false)
    (Variables|Default|SetButtonCurrentLocation (- (Variables|Default|GetButtonInitialLocation) (* (Math|Vector|GetUpVector (Variables|Default|GetButton)) (Variables|Default|GetCurrentButtonTravel))))
    (if (>= (Variables|Default|GetCurrentButtonTravel) (Variables|Default|GetMaximumButtonTravel))
      (CallFunction|FullyPressed))
    (elif (Variables|Default|GetbIsReturning)
      (bind _output_get (Variables|Default|SetButtonCurrentLocation (Math|Interpolation|VInterpTo (Variables|Default|GetButtonCurrentLocation) (Variables|Default|GetButtonInitialLocation) (Utilities|Time|GetWorldDeltaSeconds) (Variables|Default|GetButtonReturnSpeed))))
      (Transformation|SetWorldLocation (Variables|Default|GetButton) _output_get false false)
      (if (Class|KismetMathLibrary|EqualExactlyVectorVector (Variables|Default|GetButtonCurrentLocation) (Variables|Default|GetButtonInitialLocation))
        (Variables|Default|SetbIsReturning false)
        (Rendering|Material|SetScalarParameterValue (Variables|Default|GetMaterialInstanceButton) "Glow" 1.0 :!class /Script/Engine.MaterialInstanceDynamic)))))

(event EventBeginPlay
  (bind _returnvalue (Rendering|Material|CreateDynamicMaterialInstance (Variables|Default|GetButton) 0 "/Game/Blueprints/Button/Button.Button" "None" :!class /Script/Engine.PrimitiveComponent))
  (Variables|Default|SetMaterialInstanceButton _returnvalue))

(fn ConstructionScript)