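; Magic carpet vehicle for VR that carries a MotionControllerPawn and is steered by lever values.
; Side and forward lever events scale their values into yaw and forward rates, which Tick applies as local rotation and offset along the Cube's forward vector, without delta-time scaling or sweep.
; Box overlap snap-attaches the pawn and detaches it on exit, setting PlayerOnVehicle, which does not gate movement.
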(event OnComponentBeginOverlap(Box)
  (params (OverlappedComponent :type Primitive%20Component%20Object%20Reference) (OtherActor :type Actor%20Object%20Reference) (OtherComp :type Primitive%20Component%20Object%20Reference) (OtherBodyIndex :type Integer) (bFromSweep :type Boolean) (SweepResult :type Hit%20Result%20Structure%20%28by%20ref%29))
  (bind _asmotion_controller_pawn (Utilities|Casting|CastToMotionControllerPawn OtherActor))
  (Transformation|AttachActorToActor _asmotion_controller_pawn self "None" "SnapToTarget" "SnapToTarget" "SnapToTarget" true)
  (Variables|Default|SetPlayerOnVehicle true))

(event OnComponentEndOverlap(Box)
  (params (OverlappedComponent :type Primitive%20Component%20Object%20Reference) (OtherActor :type Actor%20Object%20Reference) (OtherComp :type Primitive%20Component%20Object%20Reference) (OtherBodyIndex :type Integer))
  (bind _asmotion_controller_pawn (Utilities|Casting|CastToMotionControllerPawn OtherActor))
  (Transformation|DetachFromActor _asmotion_controller_pawn "KeepRelative" "KeepRelative" "KeepRelative")
  (Variables|Default|SetPlayerOnVehicle false))

(event EventBeginPlay)

(event Collision|EventActorBeginOverlap
  (params (OtherActor :type Actor%20Object%20Reference)))

(event EventTick
  (params (DeltaSeconds :type Float%20%28single-precision%29))
  (Transformation|AddActorLocalOffset (* (Math|Vector|GetForwardVector (Variables|Default|GetCube)) (Variables|Default|GetForwardRate)) false false)
  (Transformation|AddActorLocalRotation (Math|Rotator|MakeRotator 0.0 0.0 (Variables|Default|GetRotationRate)) false false))

(event EventSideValueChange
  (params (LeverValue :type Float%20%28single-precision%29))
  (Variables|Default|SetRotationRate (* LeverValue (Variables|Default|GetRotationMultiplier))))

(event EventForwardValueChange
  (params (LeverValue :type Float%20%28single-precision%29))
  (Variables|Default|SetForwardRate (* LeverValue (Variables|Default|GetForwardMultiplier))))

(fn ConstructionScript)