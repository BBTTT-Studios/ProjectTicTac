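; BP_Lever is a physics lever that drives a linked object and switches between button, toggle and return-to-center modes when used.
; Each tick retargets the constraint's angular drive to hold, snap or center the handle, based on mode.
; Button and toggle call I_Use on the linked object whenever the handle crosses center.
; Return-to-center sends clamped handle pitch as a forward or sideways value, displayed as text.
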(event EventBeginPlay)

(event Collision|EventActorBeginOverlap
  (params (OtherActor :type Actor%20Object%20Reference)))

(event EventTick
  (params (DeltaSeconds :type Float%20%28single-precision%29))
  (bind _returnvalue (Transformation|GetActorTransform))
  (bind _handle (Variables|Default|GetHandle))
  (bind _linkedobject (Variables|Default|GetLinkedObject))
  (bind _levertype (Variables|Default|GetLeverType))
  (bind _returnvalue_2 (Transformation|GetWorldRotation _handle))
  (bind _returnvalue_3 (Math|Transform|InverseTransformRotation _returnvalue _returnvalue_2))
  (bind _pitch (Math|Rotator|BreakRotator _returnvalue_3))
  (bind _returnvalue_4 (< _pitch 0.0))
  (Rendering|Components|TextRender|SetText (Variables|Default|GetLever%20Type) (Utilities|Text|ToText(String) (Utilities|String|EnumtoString _levertype)))
  (switch Utilities|FlowControl|Switch|SwitchonE_LeverType _levertype
    (:NewEnumerator0
      (Class|PhysicsConstraintComponent|SetAngularOrientationTarget (Variables|Default|GetPhysicsConstraint) (Math|Rotator|MakeRotator 0.0 45.0 0.0))
      (Rendering|SetVisibility (Variables|Default|GetLever%20Progress) false false :!label _label)
      (Class|PhysicsConstraintComponent|SetAngularDriveParams (Variables|Default|GetPhysicsConstraint) 3e+03 0.0 0.0)
      (if (Math|Boolean|NotEqual(Boolean) (Variables|Default|GetIsOn) _returnvalue_4)
        (Variables|Default|SetIsOn _returnvalue_4)
        (bind _asi_use (Utilities|Casting|CastToI_Use (Variables|Default|GetLinkedObject)))
        (Default|Use _asi_use)
        (if (Variables|Default|GetIsOn)
          (Audio|PlaySoundatLocation "/Game/Blueprints/Button/Boop.Boop" (Transformation|GetWorldLocation (Variables|Default|GetDefaultSceneRoot)) "0, 0, 0" 1.0 1.0 0.0 0 0 0))))
    (:NewEnumerator1
      (Class|PhysicsConstraintComponent|SetAngularOrientationTarget (Variables|Default|GetPhysicsConstraint) (Math|Rotator|MakeRotator 0.0 (select _returnvalue_4 -45.0 45.0) 0.0))
      (goto _label))
    (:NewEnumerator2
      (Class|PhysicsConstraintComponent|SetAngularOrientationTarget (Variables|Default|GetPhysicsConstraint) (Math|Rotator|MakeRotator 0.0 0.0 0.0))
      (Rendering|SetVisibility (Variables|Default|GetLever%20Progress) true false)
      (Class|PhysicsConstraintComponent|SetAngularDriveParams (Variables|Default|GetPhysicsConstraint) 3e+08 0.0 0.0)
      (bind _output_get (Variables|Default|SetLeverProgress (Math|Float|Clamp(Float) (- (* (/ (+ _pitch 45.0) 9e+01) 2e+02) 1e+02) -1e+02 1e+02)))
      (Rendering|Components|TextRender|SetText (Variables|Default|GetLever%20Progress) (Utilities|Text|ToText(Float) _output_get "HalfToEven"))
      (switch Utilities|FlowControl|Switch|SwitchonE_LeverDirection (Variables|Default|GetLeverDirection)
        (:NewEnumerator0
          (Class|IAxisLever|ForwardValueChange(Message) _linkedobject (Variables|Default|GetLeverProgress)))
        (:NewEnumerator1
          (Class|IAxisLever|SideValueChange(Message) _linkedobject (Variables|Default|GetLeverProgress)))))))

(event EventUse
  (switch Utilities|FlowControl|Switch|SwitchonE_LeverType (Variables|Default|GetLeverType)
    (:NewEnumerator0
      (Variables|Default|SetLeverType "NewEnumerator1"))
    (:NewEnumerator1
      (Variables|Default|SetLeverType "NewEnumerator2"))
    (:NewEnumerator2
      (Variables|Default|SetLeverType "NewEnumerator0"))))

(fn ConstructionScript
  (Utilities|FlowControl|Sequence
    (:then_0
      (Rendering|SetVisibility (Variables|Default|GetLever%20Type) (Variables|Default|GetShowLeverType) false))
    (:then_1
      (Rendering|SetVisibility (Variables|Default|GetLever%20Progress) (Variables|Default|GetShowLeverProgress) false))))