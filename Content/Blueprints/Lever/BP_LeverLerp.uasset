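; BP_LeverLerp is a lever actor that turns the angle of its handle into a progress value and displays it.
; Every tick it converts the Handle's world rotation into actor space and linearly remaps pitch from ±45 degrees to a clamped ±100 range.
; The result is stored in LeverProgress and written to the LeverProgressText component.
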(event EventBeginPlay)

(event Collision|EventActorBeginOverlap
  (params (OtherActor :type Actor%20Object%20Reference)))

(event EventTick
  (params (DeltaSeconds :type Float%20%28single-precision%29))
  (bind _output_get (Variables|Default|SetLeverProgress (Math|Float|Clamp(Float) (- (* (/ (+ (.Pitch (Math|Rotator|BreakRotator (Math|Transform|InverseTransformRotation (Transformation|GetActorTransform) (Transformation|GetWorldRotation (Variables|Default|GetHandle))))) 45.0) 9e+01) 2e+02) 1e+02) -1e+02 1e+02)))
  (Rendering|Components|TextRender|SetText (Variables|Default|GetLeverProgressText) (Utilities|Text|ToText(Float) _output_get "HalfToEven")))

(fn ConstructionScript)