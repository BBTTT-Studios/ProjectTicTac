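; Lever actor that triggers a linked object whenever its handle crosses the level position.
; Each tick it converts the Handle's world rotation into actor space and treats negative pitch as on.
; When that state differs from IsOn, it stores the new value and calls Use on LinkedObject through the I_Use interface, in both directions.
; The graph itself contains no snapping or one-way logic.
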(event EventBeginPlay)

(event Collision|EventActorBeginOverlap
  (params (OtherActor :type Actor%20Object%20Reference)))

(event EventTick
  (params (DeltaSeconds :type Float%20%28single-precision%29))
  (bind _returnvalue (Transformation|GetActorTransform))
  (bind _handle (Variables|Default|GetHandle))
  (bind _returnvalue_2 (Transformation|GetWorldRotation _handle))
  (bind _returnvalue_3 (Math|Transform|InverseTransformRotation _returnvalue _returnvalue_2))
  (bind _pitch (Math|Rotator|BreakRotator _returnvalue_3))
  (bind _returnvalue_4 (< _pitch 0.0))
  (if (Math|Boolean|NotEqual(Boolean) (Variables|Default|GetIsOn) _returnvalue_4)
    (Variables|Default|SetIsOn _returnvalue_4)
    (bind _asi_use (Utilities|Casting|CastToI_Use (Variables|Default|GetLinkedObject)))
    (Default|Use _asi_use)))

(fn ConstructionScript)