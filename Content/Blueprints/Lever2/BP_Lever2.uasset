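; VR lever that a motion controller grabs and pulls to trigger a linked object.
; While held, Tick converts the interactor's position into local space and uses a clamped Atan2 angle to rotate the lever.
; When the ball overlaps FinalPullBox, the lever resets and calls I_Use on LinkedObject; release also resets it through a timeline lerp.
; GetClosestComponentData supplies the closest grab point on the ball.
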(event OnComponentBeginOverlap(FinalPullBox)
  (params (OverlappedComponent :type Primitive%20Component%20Object%20Reference) (OtherActor :type Actor%20Object%20Reference) (OtherComp :type Primitive%20Component%20Object%20Reference) (OtherBodyIndex :type Integer) (bFromSweep :type Boolean) (SweepResult :type Hit%20Result%20Structure%20%28by%20ref%29))
  (bind _linkedobject (Variables|Default|GetLinkedObject))
  ;[1 1 1] Detect lever pull
  (if (== OtherComp (Variables|Default|GetLeverBall))
    (CallFunction|ResetRotation)
    (Utilities|IsValid _linkedobject
      (:Is%20Valid
        (bind _asi_use (Utilities|Casting|CastToI_Use _linkedobject))
        (Default|Use _asi_use)
        (Utilities|IsValid (Variables|Default|GetCurrentInteractor))))))

(event Custom|ResetRotation
  (Variables|Default|SetResettingRotation true)
  (Variables|Default|SetInterpLeverRotation (Variables|/Script/Engine.SceneComponent|GetRelativeRotation (Variables|Default|GetLeverRotate)))
  (bind _alpha (Timeline|Timeline_0 PlayFromStart)
    (:Update
      (Transformation|SetRelativeRotation (Variables|Default|GetLeverRotate) (Math|Rotator|Lerp(Rotator) (Variables|Default|GetInterpLeverRotation) (Variables|Default|GetInitialLeverRotation) _alpha) false false)
      (Variables|Default|SetCurrentInteractor 0))
    (:Finished
      (Variables|Default|SetResettingRotation false))))

(event EventBeginPlay
  (Variables|Default|SetInitialLeverRotation (Variables|/Script/Engine.SceneComponent|GetRelativeRotation (Variables|Default|GetLeverRotate))))

(event EventTick
  (params (DeltaSeconds :type Float%20%28single-precision%29))
  (bind _returnvalue (Transformation|GetActorTransform))
  (bind _leverrotate (Variables|Default|GetLeverRotate))
  (bind _currentinteractor (Variables|Default|GetCurrentInteractor))
  (bind _currentinteractor_2 (Variables|Default|GetCurrentInteractor))
  (bind _returnvalue_2 (Transformation|GetWorldLocation _currentinteractor))
  (bind _relativelocation (Variables|/Script/Engine.SceneComponent|GetRelativeLocation _leverrotate))
  (bind _returnvalue_3 (Math|Transform|InverseTransformLocation _returnvalue _returnvalue_2))
  (bind _returnvalue_4 (- _returnvalue_3 _relativelocation))
  (Utilities|IsValid _currentinteractor_2
    (:Is%20Valid
      (bind _asbp_motion_controller (Utilities|Casting|CastToBP_MotionController (Components|GetOwner _currentinteractor_2)))
      (if (== (Variables|/Game/VirtualRealityBP/Blueprints/BP_MotionController.BP_MotionController_C|GetAttachedActor _asbp_motion_controller) self)
        (if (not (Variables|Default|GetResettingRotation))
          (Transformation|SetRelativeRotation (Variables|Default|GetLeverRotate) (Math|Rotator|MakeRotator 0.0 0.0 (Math|Float|Clamp(Float) (Class|KismetMathLibrary|DegAtan2 (.z _returnvalue_4) (.x _returnvalue_4)) (Variables|Default|GetMinPitch) (Variables|Default|GetMaxPitch))) false false))
        (else
          (CallFunction|ResetRotation))))))

(event EventPickup
  (params (Interactor :type Scene%20Component%20Object%20Reference))
  (bind _output_get (Variables|Default|SetCurrentInteractor Interactor))
  (bind _asbp_motion_controller (Utilities|Casting|CastToBP_MotionController (Components|GetOwner _output_get)))
  (Variables|/Game/VirtualRealityBP/Blueprints/BP_MotionController.BP_MotionController_C|SetAttachedActor _asbp_motion_controller self))

(fn ConstructionScript)

(fn GetClosestComponentData
  (params (Interactor :type Scene%20Component%20Object%20Reference))
  (return (.OutPointOnBody (Collision|GetClosestPointonCollision (Variables|Default|GetLeverBall) (Transformation|GetWorldLocation Interactor) "None")) 0 (Variables|Default|GetLeverBall)))