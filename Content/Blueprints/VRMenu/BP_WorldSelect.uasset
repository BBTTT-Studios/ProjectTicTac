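; BP_WorldSelect is a VR menu Blueprint that exposes a map selection widget for choosing a world.
; Its Up and Down events cast the Widget component's user widget to MapSelect and move the selection.
; Tick repeats the cast every frame to copy the widget's SelectedMap into the Blueprint's MapName variable.
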(event Custom|Up
  (bind _asmap_select (Utilities|Casting|CastToMapSelect (UserInterface|GetUserWidgetObject (Variables|Default|GetWidget))))
  (Default|SelectionUp _asmap_select))

(event Custom|Down
  (bind _asmap_select (Utilities|Casting|CastToMapSelect (UserInterface|GetUserWidgetObject (Variables|Default|GetWidget))))
  (Default|SelectionDown _asmap_select))

(event EventBeginPlay)

(event Collision|EventActorBeginOverlap
  (params (OtherActor :type Actor%20Object%20Reference)))

(event EventTick
  (params (DeltaSeconds :type Float%20%28single-precision%29))
  (bind _asmap_select (Utilities|Casting|CastToMapSelect (UserInterface|GetUserWidgetObject (Variables|Default|GetWidget))))
  (Variables|Default|SetMapName (Variables|/Game/Blueprints/VRMenu/MapSelect.MapSelect_C|GetSelectedMap _asmap_select)))

(fn ConstructionScript)