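; BP_SnapTile is a labeled tile that can be picked up, carried and snapped into BP_TileReceptacle actors.
; Pickup attaches it to a given component, while Cube overlap events track the receptacle whose Box it touches.
; Drop detaches it and, if a receptacle is tracked, attaches and aligns it there with a slight upward offset.
; The Construction Script and a RefreshText event set its label from TileText.
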(event OnComponentBeginOverlap(Cube)
  (params (OverlappedComponent :type Primitive%20Component%20Object%20Reference) (OtherActor :type Actor%20Object%20Reference) (OtherComp :type Primitive%20Component%20Object%20Reference) (OtherBodyIndex :type Integer) (bFromSweep :type Boolean) (SweepResult :type Hit%20Result%20Structure%20%28by%20ref%29))
  (bind _asbp_tile_receptacle (Utilities|Casting|CastToBP_TileReceptacle OtherActor))
  (if (== (Variables|/Game/Blueprints/SnapTiles/BP_TileReceptacle.BP_TileReceptacle_C|GetBox _asbp_tile_receptacle) OtherComp)
    (Variables|Default|SetOverlappedReceptacle _asbp_tile_receptacle)))

(event OnComponentEndOverlap(Cube)
  (params (OverlappedComponent :type Primitive%20Component%20Object%20Reference) (OtherActor :type Actor%20Object%20Reference) (OtherComp :type Primitive%20Component%20Object%20Reference) (OtherBodyIndex :type Integer))
  (bind _asbp_tile_receptacle (Utilities|Casting|CastToBP_TileReceptacle OtherActor))
  (if (== (Variables|/Game/Blueprints/SnapTiles/BP_TileReceptacle.BP_TileReceptacle_C|GetBox _asbp_tile_receptacle) OtherComp)
    (Variables|Default|SetOverlappedReceptacle 0)))

(event Custom|RefreshText
  (Rendering|Components|TextRender|SetText (Variables|Default|GetText) (Utilities|Text|ToText(String) (Variables|Default|GetTileText))))

(event EventBeginPlay)

(event Collision|EventActorBeginOverlap
  (params (OtherActor :type Actor%20Object%20Reference)))

(event EventPickup
  (params (AttachTo :type Scene%20Component%20Object%20Reference))
  (Transformation|DetachFromActor "KeepWorld" "KeepWorld" "KeepWorld")
  (Variables|Default|SetIsHeld true)
  (Transformation|AttachComponentToComponent (VehicleSound|GetRootComponent) AttachTo "None" "KeepWorld" "KeepWorld" "KeepWorld" false))

(event EventDrop
  (Variables|Default|SetIsHeld false)
  (Transformation|DetachFromActor "KeepWorld" "KeepWorld" "KeepWorld")
  (Utilities|IsValid (Variables|Default|GetOverlappedReceptacle)
    (:Is%20Valid
      (Transformation|AttachActorToActor (Variables|Default|GetOverlappedReceptacle) "None" "SnapToTarget" "SnapToTarget" "KeepWorld" true)
      (Transformation|AddActorWorldOffset "0, 0,3.000000"))))

(fn ConstructionScript
  (Rendering|Components|TextRender|SetText (Variables|Default|GetText) (Utilities|Text|ToText(String) (Variables|Default|GetTileText))))