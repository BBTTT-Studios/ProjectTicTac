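; BP_TileHolder builds a row of letter receptacles for a word puzzle, one per letter of TargetWord.
; InitializeBoxes spawns BP_TileReceptacle child actors under TileAnchor, shifting and re-indexing existing ones after each addition, at BeginPlay or in construction when Preview is on.
; Tick prepends each receptacle's letter, or an underscore if empty, into GuessedWord, which the TextRender shows a frame later.
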(event Custom|InitializeBoxes
  ;[1 1 1] Clear all previous tiles
  (for _array_element (Variables|Default|GetHolderInstances)
    (Actor|DestroyActor _array_element))
  (Variables|Default|SetPreviousBoxTransform "")
  ;[1 1 1] Run once for each letter in target word
  (for _index (range 1 (Utilities|String|Len (Variables|Default|GetTargetWord)))
    ;[1 1 1] Create an instance of tile holder at an offset based on the previous tile and the Tile Spacing variable
    (bind _returnvalue (AddComponent|AddChildActorComponent false (Math|Transform|MakeTransform (Math|Vector|MakeVector (.X (Math|Vector|BreakVector (.location (Variables|Default|GetPreviousBoxTransform)))) (+ (.Y (Math|Vector|BreakVector (.location (Variables|Default|GetPreviousBoxTransform)))) (Variables|Default|GetTileSpacing)) (.Z (Math|Vector|BreakVector (.location (Variables|Default|GetPreviousBoxTransform))))) "0, 0, 0" "1,1,1")))
    ;[1 1 1] Add tile holder instance to an array and attach to the TileAnchor component
    (bind _asbp_tile_receptacle (Utilities|Casting|CastToBP_TileReceptacle (Variables|/Script/Engine.ChildActorComponent|GetChildActor _returnvalue)))
    (Utilities|Array|Add (Variables|Default|GetHolderInstances) _asbp_tile_receptacle)
    (Transformation|AttachComponentToComponent _returnvalue (Variables|Default|GetTileAnchor) "None" "KeepRelative" "KeepRelative" "KeepWorld" true)
    (Variables|Default|SetPreviousBoxTransform (Transformation|GetRelativeTransform _returnvalue))
    (for (_array_element_2 _array_index) (Variables|Default|GetHolderInstances)
      (Utilities|IsValid _array_element_2
        (:Is%20Valid
          (Transformation|AddLocalOffset (Variables|/Script/Engine.Actor|GetRootComponent _array_element_2) (Math|Vector|MakeVector 0.0 (+ (* (Variables|Default|GetTileSpacing) -2.0) (Variables|Default|GetTileSpacing)) 0.0) false false)
          (Variables|/Game/Blueprints/SnapTiles/BP_TileReceptacle.BP_TileReceptacle_C|SetIndex _array_element_2 _array_index))))))

(event EventBeginPlay
  (CallFunction|InitializeBoxes))

(event EventTick
  (params (DeltaSeconds :type Float%20%28single-precision%29))
  (Rendering|Components|TextRender|SetText (Variables|Default|GetTextRender) (Utilities|Text|ToText(String) (Variables|Default|GetGuessedWord)))
  (Variables|Default|SetGuessedWord "")
  (for _array_element (Variables|Default|GetHolderInstances)
    (Utilities|IsValid _array_element
      (:Is%20Valid
        (if (not (Utilities|Enum|Equal(Enum) (Variables|/Game/Blueprints/SnapTiles/BP_TileReceptacle.BP_TileReceptacle_C|GetText _array_element) ""))
          (Variables|Default|SetGuessedWord (Utilities|String|Append (Variables|/Game/Blueprints/SnapTiles/BP_TileReceptacle.BP_TileReceptacle_C|GetText _array_element) (Variables|Default|GetGuessedWord)))
          (else
            (Variables|Default|SetGuessedWord (Utilities|String|Append "_" (Variables|Default|GetGuessedWord)))))))))

(fn ConstructionScript
  (if (Variables|Default|GetPreview)
    (CallFunction|InitializeBoxes)))