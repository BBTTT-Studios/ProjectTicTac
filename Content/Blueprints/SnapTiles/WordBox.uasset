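; WordBox is an overlap actor for a snap-tile spelling puzzle that checks spelt words against a pedestal's prompt.
; On each overlap, it appends the display names of all overlapping BP_SnapTile actors to SpeltWord without clearing it first.
; It casts its owner to BP_Pedestal and compares the word with CurrentPrompt, printing success on a match or destroying the newly overlapping actor otherwise.
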(event Collision|EventActorBeginOverlap
  (params (OtherActor :type Actor%20Object%20Reference))
  (for _array_element (Collision|GetOverlappingActors "/Game/Blueprints/SnapTiles/BP_SnapTile.BP_SnapTile_C" :!class /Script/Engine.Actor)
    (bind _output_get (Variables|Default|SetSpeltWord (Utilities|String|Append (stale _output_get) (Utilities|GetDisplayName _array_element))))
    (Development|PrintString _output_get))
  (bind _asbp_pedestal (Utilities|Casting|CastToBP_Pedestal (Components|GetOwner))
    (:then
      (if (Utilities|Enum|Equal(Enum) (Variables|/Game/DrawingPrompt/BP_Pedestal.BP_Pedestal_C|GetCurrentPrompt _asbp_pedestal) (Variables|Default|GetSpeltWord))
        (Development|PrintString "Success!")
        (else
          (Actor|DestroyActor OtherActor))))
    (:CastFailed
      (Development|PrintString (Variables|/Game/DrawingPrompt/BP_Pedestal.BP_Pedestal_C|GetCurrentPrompt _asbp_pedestal)))))

(fn ConstructionScript)