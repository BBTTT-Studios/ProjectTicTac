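; B_Light is an interactable point light that can be switched on and off or dimmed by a lever value.
; The Use event flips the Lit flag and applies it to the PointLight's visibility.
; ForwardValueChange remaps the signed lever value linearly to intensity and forces the light visible.
; Both branches of its intensity check set Lit to true, so the flag stays on even at zero intensity.
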(event EventBeginPlay)

(event Collision|EventActorBeginOverlap
  (params (OtherActor :type Actor%20Object%20Reference)))

(event EventTick
  (params (DeltaSeconds :type Float%20%28single-precision%29)))

(event EventUse
  (bind _output_get (Variables|Default|SetLit (not (Variables|Default|GetLit))))
  (Rendering|SetVisibility (Variables|Default|GetPointLight) _output_get false))

(event EventForwardValueChange
  (params (LeverValue :type Float%20%28single-precision%29))
  (Variables|Default|SetLightIntensity (Math|Float|Lerp 0.0 5e+03 (/ (+ LeverValue 1e+02) 2e+02)))
  (Rendering|SetVisibility (Variables|Default|GetPointLight) true false)
  (Rendering|Components|Light|SetIntensity (Variables|Default|GetPointLight) (Variables|Default|GetLightIntensity))
  (if (> (Variables|Default|GetLightIntensity) 0.0)
    (Variables|Default|SetLit true)
    (else
      (Variables|Default|SetLit true))))

(fn ConstructionScript)