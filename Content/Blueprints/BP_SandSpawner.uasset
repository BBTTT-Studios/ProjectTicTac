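; BP_SandSpawner is an actor that spawns a pile of tiny BP_PickupCube actors, presumably as sand grains, when its Use event fires.
; A loop over SpawnAmount places each scaled-down cube at a small random offset around the root, adjusting for collisions but always spawning.
; A short Delay ends each loop body, with nothing chained after it.
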(event EventBeginPlay)

(event Collision|EventActorBeginOverlap
  (params (OtherActor :type Actor%20Object%20Reference)))

(event EventTick
  (params (DeltaSeconds :type Float%20%28single-precision%29)))

(event EventUse
  (bind _defaultsceneroot (Variables|Default|GetDefaultSceneRoot))
  (bind _returnvalue (Transformation|GetWorldLocation _defaultsceneroot))
  (for _index (range 0 (Variables|Default|GetSpawnAmount))
    (Game|SpawnActorfromClass "/Game/VirtualRealityBP/Blueprints/BP_PickupCube.BP_PickupCube_C" (Math|Transform|MakeTransform (Math|Vector|MakeVector (+ (.x _returnvalue) (Math|Random|RandomFloatinRange -1e+01 1e+01)) (+ (.y _returnvalue) (Math|Random|RandomFloatinRange -1e+01 1e+01)) (+ (.z _returnvalue) (Math|Random|RandomFloatinRange -1e+01 1e+01))) "0, 0, 0" "0.050000,0.050000,0.050000") "AdjustIfPossibleButAlwaysSpawn" 0 0)
    (Utilities|FlowControl|Delay 0.01)))

(fn ConstructionScript)