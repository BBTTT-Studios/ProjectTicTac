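; BP_PromptStandin is a motion-controller grabbable physics prop that shows a random drawing prompt material when moving fast.
; Tick checks the mesh's linear velocity against a speed range and calls ChangeColor through a DoOnce that resets after a short delay.
; ChangeColor applies a random PromptArray entry to the mesh.
; BP_MotionController calls Pickup to disable physics and attach the actor, while Drop detaches it and restores physics.
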(event EventTick
  (params (DeltaSeconds :type Float%20%28single-precision%29))
  (if true
    (bind _returnvalue (Physics|GetPhysicsLinearVelocity (Variables|Default|GetStaticMesh) "None"))
    (if (Math|Float|InRange(Float) (Math|Vector|VectorLength _returnvalue) 5e+02 1e+04)
      (Utilities|FlowControl|DoOnce false :!label _label
        (:Completed
          (CallFunction|ChangeColor)
          (Utilities|FlowControl|Delay 2.0)
          (goto _label Reset))))))

(event EventPickup
  (params (AttachTo :type Scene%20Component%20Object%20Reference))
  (Variables|Default|SetIsHeld true)
  (Physics|SetSimulatePhysics (Variables|Default|GetStaticMesh) false)
  (Transformation|AttachComponentToComponent (VehicleSound|GetRootComponent) AttachTo "None" "KeepWorld" "KeepWorld" "KeepWorld" false))

(event EventDrop
  (Variables|Default|SetIsHeld false)
  (Physics|SetSimulatePhysics (Variables|Default|GetStaticMesh) true)
  (Transformation|DetachFromActor "KeepWorld" "KeepWorld" "KeepWorld"))

(fn ConstructionScript)

(fn ChangeColor
  (bind _promptarray (Variables|Default|GetPromptArray))
  (Rendering|Material|SetMaterial (Variables|Default|GetStaticMesh) 0 (Utilities|Array|Get(acopy) _promptarray (Math|Random|RandomInteger (+ (Utilities|Array|LastIndex _promptarray) 1)))))